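; LightButtonSwitch is an interactable button that switches a set of lights, with a tries counter tracking presses.
; A box overlap with ThirdPersonCharacter enables the button's input, and leaving the box disables it.
; Releasing E plays a sound, calls SwitchLight on every actor in LightActors, then calls IsOnCheck and CountTries on the TriesCounter actor found by class lookup.
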(event OnComponentBeginOverlap(Box)
  (params (OverlappedComponent :type Primitive%20Component%20Object%20Reference) (OtherActor :type Actor%20Object%20Reference) (OtherComp :type Primitive%20Component%20Object%20Reference) (OtherBodyIndex :type Integer) (bFromSweep :type Boolean) (SweepResult :type Hit%20Result%20Structure%20%28by%20ref%29))
  (Utilities|Casting|CastToThirdPersonCharacter OtherActor)
  (Input|EnableInput (Game|GetPlayerController 0)))

(event OnComponentEndOverlap(Box)
  (params (OverlappedComponent :type Primitive%20Component%20Object%20Reference) (OtherActor :type Actor%20Object%20Reference) (OtherComp :type Primitive%20Component%20Object%20Reference) (OtherBodyIndex :type Integer))
  (Utilities|Casting|CastToThirdPersonCharacter OtherActor)
  (Input|DisableInput (Game|GetPlayerController 0)))

(event Input|KeyboardEvents|E
  (params (Key :type Key%20Structure :default "None"))
  (:Released
    (Audio|PlaySoundatLocation "/Game/Ivan/Blueprints/ButtonLitSound.ButtonLitSound" (Transformation|GetActorLocation) "0, 0, 0" 1.0 1.0 0.0 0 0 0)
    (for _array_element (Variables|Default|GetLightActors)
      (Default|SwitchLight _array_element))
    (bind _returnvalue (Actor|GetActorOfClass "/Game/Ivan/Blueprints/TriesCounter.TriesCounter_C"))
    (Default|IsonCheck _returnvalue)
    (bind _returnvalue_2 (Actor|GetActorOfClass "/Game/Ivan/Blueprints/TriesCounter.TriesCounter_C"))
    (Default|CountTries _returnvalue_2)))

(fn ConstructionScript)