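; An elevator platform actor that the player operates by key press while standing in its trigger box.
; ThirdPersonCharacter entering or leaving the Box enables or disables the actor's input for player controller 0.
; E plays PlatformTimeline and F reverses it.
; The timeline's MoveElevator track sets ShapeCube's relative location on each update, without sweep.
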(event OnComponentBeginOverlap(Box)
  (params (OverlappedComponent :type Primitive%20Component%20Object%20Reference) (OtherActor :type Actor%20Object%20Reference) (OtherComp :type Primitive%20Component%20Object%20Reference) (OtherBodyIndex :type Integer) (bFromSweep :type Boolean) (SweepResult :type Hit%20Result%20Structure%20%28by%20ref%29))
  ;[1 1 1] Moving Platform
  (Utilities|Casting|CastToThirdPersonCharacter OtherActor)
  (Input|EnableInput (Game|GetPlayerController 0)))

(event OnComponentEndOverlap(Box)
  (params (OverlappedComponent :type Primitive%20Component%20Object%20Reference) (OtherActor :type Actor%20Object%20Reference) (OtherComp :type Primitive%20Component%20Object%20Reference) (OtherBodyIndex :type Integer))
  ;[1 1 1] Moving Platform
  (Utilities|Casting|CastToThirdPersonCharacter OtherActor)
  (Input|DisableInput (Game|GetPlayerController 0)))

(event EventBeginPlay)

(event Collision|EventActorBeginOverlap
  (params (OtherActor :type Actor%20Object%20Reference)))

(event EventTick
  (params (DeltaSeconds :type Float%20%28single-precision%29)))

(event Input|KeyboardEvents|E
  (params (Key :type Key%20Structure))
  ;[1 1 1] Moving Platform
  (:Pressed
    (bind _move_elevator (Timeline|Platform%20Timeline Play)
      (:Update
        (Transformation|SetRelativeLocation (Variables|Default|GetShape_Cube) _move_elevator false false)))))

(event Input|KeyboardEvents|F
  (params (Key :type Key%20Structure))
  ;[1 1 1] Moving Platform
  (:Pressed
    (bind _move_elevator (Timeline|Platform%20Timeline Reverse)
      (:Update
        (Transformation|SetRelativeLocation (Variables|Default|GetShape_Cube) _move_elevator false false)))))

(fn ConstructionScript)