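; Keycard-locked elevator door that opens when a third person character carrying the matching key enters its trigger box.
; The overlap checks the character's KeyCollection at KeyValue, then either slides the mesh open via a timeline with sound or briefly shows a NoKey widget.
; DoOnce gates prevent repeat triggers, and the key slot is cleared after opening for one-time use.
; The construction script sets the mesh and tints a dynamic material by colour.
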(event OnComponentBeginOverlap(Box)
  (params (OverlappedComponent :type Primitive%20Component%20Object%20Reference) (OtherActor :type Actor%20Object%20Reference) (OtherComp :type Primitive%20Component%20Object%20Reference) (OtherBodyIndex :type Integer) (bFromSweep :type Boolean) (SweepResult :type Hit%20Result%20Structure%20%28by%20ref%29))
  ;[1 1 1] Array Not used
  (bind _asthird_person_character (Utilities|Casting|CastToThirdPersonCharacter OtherActor))
  (Utilities|FlowControl|DoOnce false :!label _label
    (:Completed
      ;;[1 1 1] Checking Each key Value | Array
      ;;;[1 1 1] If they have the correct key, it will open
      (bind (_array_element _array_index) (Utilities|Array|ForEachLoopwithBreak (Variables|/Game/ThirdPersonBP/Blueprints/ThirdPersonCharacter.ThirdPersonCharacter_C|GetKey%20Collection _asthird_person_character) :!label _label_2)
        (:LoopBody
          (if (and _array_element (== _array_index (Variables|Default|GetKey%20Value)))
            (CallFunction|OpenElevator)
            (goto _label_2 Break)))
        (:Completed
          (if (not (and _array_element (== _array_index (Variables|Default|GetKey%20Value))))
            (Utilities|FlowControl|Sequence
              (:then_0
                ;;;[1 1 1] Don't havce the correct key. Will create a widget telling player that they have the incorrect key card
                (Utilities|FlowControl|DoOnce false :!label _label_3
                  (:Completed
                    (bind _returnvalue (UserInterface|CreateWidget "/Game/James/Elevators_System/NoKey_BP.NoKey_BP_C"))
                    (UserInterface|Viewport|AddtoViewport _returnvalue 0)
                    (Utilities|FlowControl|Delay 4.0)
                    (Widget|RemovefromParent _returnvalue)
                    (goto _label_3 Reset))))
              (:then_1
                (goto _label Reset)))))))))

(event Custom|Open%20Elevator
  ;[1 1 1] Comment
  ;;[1 1 1] Custom Event
  (Audio|PlaySoundatLocation "/Game/James/Elevators_System/Elvator_Open.Elvator_Open" (Transformation|GetActorLocation) "0, 0, 0" 0.25 1.0 0.8 0 0 0)
  ;;[1 1 1] Timeline
  (bind _open_elevator_track (Timeline|Elevator%20Open PlayFromStart)
    (:Update
      ;;[1 1 1] Location in correlation with the timeline (closed/open)
      (Transformation|SetRelativeLocation (Variables|Default|GetStaticMesh) (Math|Vector|Lerp(Vector) (Variables|Default|GetClose) (Variables|Default|GetOpen) _open_elevator_track) false false))
    (:Finished
      ;[1 1 1] Key one time use
      (Utilities|FlowControl|Delay 1.0)
      (Utilities|Array|SetArrayElem (Variables|/Game/ThirdPersonBP/Blueprints/ThirdPersonCharacter.ThirdPersonCharacter_C|GetKey%20Collection (stale OnComponentBeginOverlap(Box) _asthird_person_character)) (Variables|Default|GetKey%20Value) false))))

(fn ConstructionScript
  (bind _staticmesh (Variables|Default|GetStaticMesh))
  ;[1 1 1] Set Key to Different colours/floors
  (Components|StaticMesh|SetStaticMesh _staticmesh (Variables|Default|GetElevator%20Mesh))
  (bind _returnvalue (Rendering|Material|CreateDynamicMaterialInstance _staticmesh 0 (Variables|Default|GetMaterial) "None" :!class /Script/Engine.PrimitiveComponent))
  (Rendering|Material|SetVectorParameterValue _returnvalue "Colour" (Variables|Default|GetColour) :!class /Script/Engine.MaterialInstanceDynamic)
  (Rendering|Material|SetMaterial _staticmesh 0 _returnvalue))