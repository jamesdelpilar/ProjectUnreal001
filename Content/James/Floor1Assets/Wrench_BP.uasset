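; Wrench pickup that acts as a key for the ThirdPersonCharacter.
; On box overlap it inserts true into the character's KeyCollection at KeyValue and shows a Key_Pickup_BP widget tinted with KeyColour.
; It destroys its box and mesh immediately, then removes the widget and itself after a short delay.
; The construction script applies KeyMesh and a dynamic KeyMaterial instance with Colour fixed to black rather than KeyColour.
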(event OnComponentBeginOverlap(Box)
  (params (OverlappedComponent :type Primitive%20Component%20Object%20Reference) (OtherActor :type Actor%20Object%20Reference) (OtherComp :type Primitive%20Component%20Object%20Reference) (OtherBodyIndex :type Integer) (bFromSweep :type Boolean) (SweepResult :type Hit%20Result%20Structure%20%28by%20ref%29))
  ;[1 1 1] Pick up key = Set True
  (bind _asthird_person_character (Utilities|Casting|CastToThirdPersonCharacter OtherActor))
  (Utilities|Array|Insert (Variables|/Game/ThirdPersonBP/Blueprints/ThirdPersonCharacter.ThirdPersonCharacter_C|GetKey%20Collection _asthird_person_character) true (Variables|Default|GetKey%20Value))
  ;[1 1 1] Tells player that we have the right key
  (bind _returnvalue (UserInterface|CreateWidget "/Game/James/Elevators_System/Key_Pickup_BP.Key_Pickup_BP_C"))
  (Variables|/Game/James/Elevators_System/Key_Pickup_BP.Key_Pickup_BP_C|SetColour _returnvalue (Variables|Default|GetKey%20Colour))
  (UserInterface|Viewport|AddtoViewport _returnvalue 0)
  (Components|DestroyComponent (Variables|Default|GetBox))
  (Utilities|FlowControl|Delay 3.0)
  (Widget|RemovefromParent _returnvalue)
  (Actor|DestroyActor))

(fn ConstructionScript
  (bind _staticmesh (Variables|Default|GetStaticMesh))
  (Components|StaticMesh|SetStaticMesh _staticmesh (Variables|Default|GetKey%20Mesh))
  (bind _returnvalue (Rendering|Material|CreateDynamicMaterialInstance _staticmesh 0 (Variables|Default|GetKey%20Material) "None" :!class /Script/Engine.PrimitiveComponent))
  (Rendering|Material|SetVectorParameterValue :self _returnvalue :ParameterName (Variables|Default|GetColour) :!class /Script/Engine.MaterialInstanceDynamic)
  (Rendering|Material|SetMaterial _staticmesh 0 _returnvalue))