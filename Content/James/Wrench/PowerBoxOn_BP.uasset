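; Interactive power box that the player swings open and closed with the Interact input while nearby and carrying a wrench.
; Box overlap with the third-person character enables input and opens a Gate; leaving disables input and closes it.
; A FlipFlop alternately plays and reverses a timeline that lerps the mesh yaw between closed and open angles.
; Without the wrench, pressing Interact only plays a sound at the box.
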(event OnComponentBeginOverlap(Box)
  (params (OverlappedComponent :type Primitive%20Component%20Object%20Reference) (OtherActor :type Actor%20Object%20Reference) (OtherComp :type Primitive%20Component%20Object%20Reference) (OtherBodyIndex :type Integer) (bFromSweep :type Boolean) (SweepResult :type Hit%20Result%20Structure%20%28by%20ref%29))
  ;[1 1 1] Interact with Power Box If close Enough and has wrench
  (bind _asthird_person_character (Utilities|Casting|CastToThirdPersonCharacter OtherActor))
  ;;[1 1 1] Input Interaction
  (Input|EnableInput (Game|GetPlayerController 0))
  (Utilities|FlowControl|Gate true) ; enters at Open
)

(event OnComponentEndOverlap(Box)
  (params (OverlappedComponent :type Primitive%20Component%20Object%20Reference) (OtherActor :type Actor%20Object%20Reference) (OtherComp :type Primitive%20Component%20Object%20Reference) (OtherBodyIndex :type Integer))
  ;[1 1 1] Interact with Power Box If close Enough and has wrench
  (Utilities|Casting|CastToThirdPersonCharacter OtherActor)
  ;;[1 1 1] Input Interaction
  (Input|DisableInput (Game|GetPlayerController 0))
  (Utilities|FlowControl|Gate true) ; enters at Close
)

(event Input|ActionEvents|InputActionInteract
  (params (Key :type Key%20Structure :default "None"))
  ;[1 1 1] Interact with Power Box If close Enough and has wrench
  ;;[1 1 1] If player is close to powerbox and presses "E" ...
  (:Pressed
    (if (Variables|/Game/ThirdPersonBP/Blueprints/ThirdPersonCharacter.ThirdPersonCharacter_C|GetHas%20Wrench? (stale OnComponentBeginOverlap(Box) _asthird_person_character))
      (Utilities|FlowControl|Gate true
        (:Exit
          ;[1 1 1] PowerBox On/Off
          (Utilities|FlowControl|FlipFlop
            (:A
              (bind _powerbox_track (Timeline|PowerBoxOpen/Close Play)
                (:Update
                  (Transformation|SetRelativeRotation (Variables|Default|GetStaticMesh) (Math|Rotator|MakeRotator 0.0 0.0 (Math|Float|Lerp (Variables|Default|GetClosed%20Angle) (Variables|Default|GetOpen%20Angle) _powerbox_track)) false false))))
            (:B
              (Timeline|PowerBoxOpen/Close Reverse)))))
      (else
        (Audio|PlaySoundatLocation "/Game/Ivan/Blueprints/ButtonLitSound.ButtonLitSound" (Transformation|GetActorLocation) "0, 0, 0" 1.0 1.0 0.0 0 0 0)))))

(fn ConstructionScript)